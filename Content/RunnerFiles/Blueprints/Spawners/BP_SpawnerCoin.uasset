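; Spawner Blueprint for coins that places them at its own location on a randomized timer while the level manager reports play is active.
; After finding the level manager at BeginPlay, it loops by delaying, placing a coin through the parent's SpawnActor, then rescheduling itself.
; Out-of-bounds spawned actors are destroyed.
; It also carries pickup logic: player overlap increments game mode Coins, plays a sound and destroys this actor itself.
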(event Custom|LineUpNextCoinSpawn
  (Utilities|FlowControl|Delay (Math|Random|RandomFloatinRange (Variables|Default|GetMinDelay) (Variables|Default|GetMaxDelay)))
  (CallFunction|PlaceCoin)
  (if (Variables|/Game/RunnerFiles/Blueprints/Game/BP_LevelManager.BP_LevelManager_C|GetbIsPlaying (Variables|Default|GetLevelManagerRef))
    (CallFunction|LineUpNextCoinSpawn)))

(event EventBeginPlay
  (bind (_levelmanagerfound _levelmanager) (CallFunction|GetLevelManager))
  (if _levelmanagerfound
    (Variables|Default|SetLevelManagerRef _levelmanager)
    (CallFunction|LineUpNextCoinSpawn)))

(event Collision|EventActorBeginOverlap
  (params (OtherActor :type Actor%20Object%20Reference))
  (Utilities|Casting|CastToBP_ThirdPersonCharacter OtherActor)
  (bind _asbp_third_person_game_mode (Utilities|Casting|CastToBP_ThirdPersonGameMode (Game|GetGameMode)))
  (Math|Integer|IncrementInt (Variables|/Game/RunnerFiles/Blueprints/Game/BP_ThirdPersonGameMode.BP_ThirdPersonGameMode_C|GetCoins _asbp_third_person_game_mode)
    (:%20%20
      (Audio|SpawnSound2D "/Game/Sounds/Sound_Effects/Coin_pickup.Coin_pickup" 1.0 1.0 0.0 0)
      (Actor|DestroyActor))))

(event EventSpawnedActorHitsBounds
  (params (OutOfBoundsActor :type Actor%20Object%20Reference))
  (Actor|DestroyActor OutOfBoundsActor))

(fn ConstructionScript
  (|CallParentFunction))

(fn SpawnActor
  (bind _returnvalue (|CallParentFunction))
  (return _returnvalue))

(fn PlaceCoin
  (bind _returnvalue (CallFunction|SpawnActor))
  (Transformation|SetActorLocation _returnvalue (Transformation|GetActorLocation) false false))