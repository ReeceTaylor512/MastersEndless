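; BP_SpawnerMagnet is a coin magnet pickup for the runner game, activated when BP_ThirdPersonCharacter overlaps it.
; Overlap sets the character's MagnetActive flag, shows the CoinMagnetActive widget and destroys the pickup.
; A delayed sequence then clears the flag and briefly shows CoinMagnetNotActive.
; That sequence follows DestroyActor on the same actor, so its latent delays are unlikely to complete.
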(event EventBeginPlay)

(event Collision|EventActorBeginOverlap
  (params (OtherActor :type Actor%20Object%20Reference))
  (bind _asbp_third_person_character (Utilities|Casting|CastToBP_ThirdPersonCharacter OtherActor))
  (Variables|/Game/RunnerFiles/Blueprints/ThirdPerson/BP_ThirdPersonCharacter.BP_ThirdPersonCharacter_C|SetMagnetActive _asbp_third_person_character true)
  (bind _returnvalue (UserInterface|CreateWidget "/Game/UI/OnScreenUI/CoinMagnetActive.CoinMagnetActive_C"))
  (UserInterface|Viewport|AddtoViewport _returnvalue 0)
  (Actor|DestroyActor)
  (Utilities|FlowControl|Delay 1e+01)
  (Widget|RemovefromParent _returnvalue)
  (Variables|/Game/RunnerFiles/Blueprints/ThirdPerson/BP_ThirdPersonCharacter.BP_ThirdPersonCharacter_C|SetMagnetActive _asbp_third_person_character false)
  (bind _returnvalue_2 (UserInterface|CreateWidget "/Game/UI/OnScreenUI/CoinMagnetNotActive.CoinMagnetNotActive_C"))
  (UserInterface|Viewport|AddtoViewport _returnvalue_2 0)
  (Utilities|FlowControl|Delay 5.0)
  (Widget|RemovefromParent _returnvalue_2))

(event EventTick
  (params (DeltaSeconds :type Float%20%28single-precision%29)))

(fn ConstructionScript
  (|CallParentFunction))