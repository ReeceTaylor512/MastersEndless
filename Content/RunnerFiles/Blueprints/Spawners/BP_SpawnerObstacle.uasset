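; BP_SpawnerObstacle is a runner-game spawner that places obstacles at its own location.
; On BeginPlay it caches the level manager, then schedules spawns after randomized delays, repeating while the level manager reports play is active.
; Each spawn uses the parent spawner's SpawnActor and moves the result to the spawner's position.
; Actors that hit the bounds are destroyed rather than reused.
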(event Custom|LineUpNextObstacleSpawn
  (Variables|Default|SetMinDelay (Math|Random|RandomFloatinRange 0.0 1e+01))
  (Variables|Default|SetMaxDelay (Math|Random|RandomFloatinRange 11.0 2e+01))
  (Utilities|FlowControl|Delay (Math|Random|RandomFloatinRange (Variables|Default|GetMinDelay) (Variables|Default|GetMaxDelay)))
  (CallFunction|PlaceObstacle)
  (if (Variables|/Game/RunnerFiles/Blueprints/Game/BP_LevelManager.BP_LevelManager_C|GetbIsPlaying (Variables|Default|GetLevelManagerRef))
    (CallFunction|LineUpNextObstacleSpawn)))

(event EventBeginPlay
  (bind (_levelmanagerfound _levelmanager) (CallFunction|GetLevelManager))
  (if _levelmanagerfound
    (Variables|Default|SetLevelManagerRef _levelmanager)
    (CallFunction|LineUpNextObstacleSpawn)))

(event EventSpawnedActorHitsBounds
  (params (OutOfBoundsActor :type Actor%20Object%20Reference))
  (Actor|DestroyActor OutOfBoundsActor))

(fn ConstructionScript
  (|CallParentFunction))

(fn PlaceObstacle
  (bind _returnvalue (CallFunction|SpawnActor))
  (Transformation|SetActorLocation _returnvalue (Transformation|GetActorLocation) false false))

(fn SpawnActor
  (bind _returnvalue (|CallParentFunction))
  (return _returnvalue))