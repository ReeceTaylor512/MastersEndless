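; BP_ScrollingComponent is a component that scrolls its owning actor at the level's speed, apparently for a runner game.
; BeginPlay caches the Level Manager reference, printing a message if none is found.
; Tick scales the owner's forward vector by LevelSpeed and delta time, without rechecking the reference.
; It applies that world-space vector as a local offset without sweep, so the direction of travel depends on owner rotation.
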(event EventBeginPlay
  (bind (_levelmanager _levelmanagerfound) (CallFunction|GetLevelManager))
  (if _levelmanagerfound
    (Variables|Default|SetLevelManagerRef _levelmanager)
    (else
      (Development|PrintString "No Level Manager"))))

(event EventTick
  (params (DeltaSeconds :type Float%20%28single-precision%29))
  (bind _returnvalue (Components|GetOwner))
  (bind _output_get (Variables|Default|SetDelta%20Seconds DeltaSeconds))
  (bind _output_get_2 (Variables|Default|SetMovement (* (* (Transformation|GetActorForwardVector _returnvalue) (Variables|/Game/RunnerFiles/Blueprints/Level/BP_LevelManager.BP_LevelManager_C|GetLevelSpeed (Variables|Default|GetLevelManagerRef))) _output_get)))
  (Transformation|AddActorLocalOffset _returnvalue _output_get_2 false false))