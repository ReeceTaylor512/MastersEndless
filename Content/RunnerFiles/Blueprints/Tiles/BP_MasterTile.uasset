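; Base tile for a runner game that scrolls along the world X axis each tick, scaled by delta time.
; When the third-person character overlaps its Box, it asks the game mode to spawn the next tile, then destroys itself after a short delay.
; A separate actor-overlap handler spawns an actor with no class set, offset in X from the tile's bounds, then also destroys itself after a delay.
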(event OnComponentBeginOverlap(Box)
  (params (OverlappedComponent :type Primitive%20Component%20Object%20Reference) (OtherActor :type Actor%20Object%20Reference) (OtherComp :type Primitive%20Component%20Object%20Reference) (OtherBodyIndex :type Integer) (bFromSweep :type Boolean) (SweepResult :type Hit%20Result%20Structure%20%28by%20ref%29))
  (Utilities|Casting|CastToBP_ThirdPersonCharacter OtherActor)
  (bind _asbp_third_person_game_mode (Utilities|Casting|CastToBP_ThirdPersonGameMode (Game|GetGameMode)))
  (Default|SpawnTile _asbp_third_person_game_mode)
  (Utilities|FlowControl|Delay 2.5)
  (Actor|DestroyActor))

(event EventTick
  (params (DeltaSeconds :type Float%20%28single-precision%29))
  (bind _result (Math|Float|NegateFloat (* DeltaSeconds 1e+02))
    (:%20%20
      (Transformation|AddActorWorldOffset (Math|Vector|MakeVector _result 0.0 0.0)))))

(event Collision|EventActorBeginOverlap
  (params (OtherActor :type Actor%20Object%20Reference))
  (Game|SpawnActorfromClass "BP_MasterTile_C" (Math|Transform|MakeTransform (+ (Transformation|GetActorLocation) (Math|Vector|MakeVector (* (.x (.BoxExtent (Collision|GetComponentBounds (Variables|Default|GetTile)))) 384.0) 0.0 0.0)) "0, 0, 0" "1.000000,1.000000,1.000000") "Undefined" 0 0)
  (Utilities|FlowControl|Delay 2.5)
  (Actor|DestroyActor))

(fn ConstructionScript)