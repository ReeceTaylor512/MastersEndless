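; Coin pickup for the runner game that works with the character's magnet power-up and the game mode's coin counter.
; With the magnet active, a Sphere1 overlap increments Coins, sets Used, plays a sound and destroys the coin after a delay.
; Meanwhile, a timeline moves it toward the player using VInterpTo plus a track offset.
; A Sphere overlap destroys unused coins but adds zero to the count.
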(event OnComponentBeginOverlap(Sphere1)
  (params (OverlappedComponent :type Primitive%20Component%20Object%20Reference) (OtherActor :type Actor%20Object%20Reference) (OtherComp :type Primitive%20Component%20Object%20Reference) (OtherBodyIndex :type Integer) (bFromSweep :type Boolean) (SweepResult :type Hit%20Result%20Structure%20%28by%20ref%29))
  (bind _asbp_third_person_character (Utilities|Casting|CastToBP_ThirdPersonCharacter OtherActor))
  (if (Variables|/Game/RunnerFiles/Blueprints/ThirdPerson/BP_ThirdPersonCharacter.BP_ThirdPersonCharacter_C|GetMagnetActive _asbp_third_person_character)
    (Utilities|FlowControl|Sequence
      (:then_0
        (bind _asbp_third_person_game_mode (Utilities|Casting|CastToBP_ThirdPersonGameMode (Game|GetGameMode)))
        (Math|Integer|IncrementInt (Variables|/Game/RunnerFiles/Blueprints/Game/BP_ThirdPersonGameMode.BP_ThirdPersonGameMode_C|GetCoins _asbp_third_person_game_mode)
          (:%20%20
            (Variables|Default|Setused true)
            (Audio|SpawnSound2D 0 1.0 1.0 0.0 0)
            (Utilities|FlowControl|Delay 1.0)
            (Actor|DestroyActor))))
      (:then_1
        (bind _newtrack_0 (Timeline|Timeline_0 Play)
          (:Update
            (Transformation|SetActorLocation (+ _newtrack_0 (Math|Interpolation|VInterpTo (.Location (Math|Transform|BreakTransform (Transformation|GetActorTransform))) (Transformation|GetActorLocation (Game|GetPlayerCharacter 0)) (Utilities|Time|GetWorldDeltaSeconds) 15.0)) false false)))))))

(event OnComponentBeginOverlap(Sphere)
  (params (OverlappedComponent :type Primitive%20Component%20Object%20Reference) (OtherActor :type Actor%20Object%20Reference) (OtherComp :type Primitive%20Component%20Object%20Reference) (OtherBodyIndex :type Integer) (bFromSweep :type Boolean) (SweepResult :type Hit%20Result%20Structure%20%28by%20ref%29))
  (Utilities|Casting|CastToBP_ThirdPersonCharacter OtherActor)
  (bind _asbp_third_person_game_mode (Utilities|Casting|CastToBP_ThirdPersonGameMode (Game|GetGameMode)))
  (if (not (Variables|Default|Getused))
    (Variables|/Game/RunnerFiles/Blueprints/Game/BP_ThirdPersonGameMode.BP_ThirdPersonGameMode_C|SetCoins _asbp_third_person_game_mode (+ (Variables|/Game/RunnerFiles/Blueprints/Game/BP_ThirdPersonGameMode.BP_ThirdPersonGameMode_C|GetCoins _asbp_third_person_game_mode) 0))
    (Actor|DestroyActor)))

(event EventBeginPlay)

(event Collision|EventActorBeginOverlap
  (params (OtherActor :type Actor%20Object%20Reference)))

(event EventTick
  (params (DeltaSeconds :type Float%20%28single-precision%29)))

(fn ConstructionScript)