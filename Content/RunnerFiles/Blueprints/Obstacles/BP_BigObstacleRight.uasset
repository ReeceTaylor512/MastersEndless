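; BP_BigObstacleRight is a runner-game obstacle that ends the run unless the player character is sliding through it.
; On BeginPlay, it picks a random mesh from its Obstacles array for variety.
; When BP_ThirdPersonCharacter overlaps the mesh without sliding, it calls HitObstacle on the character and GameOver on the level manager, if found.
; SetParent and ReturnParent store and expose a parent reference.
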(event OnComponentBeginOverlap(StaticMesh)
  (params (OverlappedComponent :type Primitive%20Component%20Object%20Reference) (OtherActor :type Actor%20Object%20Reference) (OtherComp :type Primitive%20Component%20Object%20Reference) (OtherBodyIndex :type Integer) (bFromSweep :type Boolean) (SweepResult :type Hit%20Result%20Structure%20%28by%20ref%29))
  (bind (_levelmanagerfound _levelmanager) (CallFunction|GetLevelManager))
  (bind _asbp_third_person_character (Utilities|Casting|CastToBP_ThirdPersonCharacter OtherActor))
  (if (not (Variables|/Game/RunnerFiles/Blueprints/ThirdPerson/BP_ThirdPersonCharacter.BP_ThirdPersonCharacter_C|GetIsSliding _asbp_third_person_character))
    (Default|HitObstacle _asbp_third_person_character)
    (if _levelmanagerfound
      (Default|GameOver _levelmanager))))

(event EventBeginPlay
  (Components|StaticMesh|SetStaticMesh (Variables|Default|GetStaticMesh) (.RandomElement (Utilities|GetRandomArrayElement (Variables|Default|GetObstacles)))))

(fn ConstructionScript)

(fn ReturnParent
  (return (Variables|Default|GetParentRef)))

(fn SetParent
  (params (Parent :type BP%20Spawner%20Base%20Object%20Reference))
  (Variables|Default|SetParentRef Parent)
  (return false))