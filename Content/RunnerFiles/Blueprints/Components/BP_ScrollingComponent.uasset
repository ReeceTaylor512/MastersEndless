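; Actor component that scrolls whatever actor owns it along the runner level, intended for floors, pickups and obstacles.
; On BeginPlay it caches the level manager through the GetLevelManager macro, printing a message if none is found.
; Each tick it applies a local offset built from the owner's forward vector, the manager's LevelSpeed and delta seconds, without sweeping or checking the cached reference.
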(event EventBeginPlay
  ;[1 1 1] This is an Actor Component, this means that it can be added to any BP Actor just like you would add a static mesh to an Actor.
  ;
  ; This class in particular is used to scroll things along the level such as the floor, pickups and obstacles
  ;;[1 0.3854 0.3854] We start with getting the level manager macro and setting a reference to this so we can use it in future classes
  (bind (_levelmanager _levelmanagerfound) (CallFunction|GetLevelManager))
  (if _levelmanagerfound
    (Variables|Default|SetLevelManagerRef _levelmanager)
    (else
      (Development|PrintString "No Level Manager"))))

(event EventTick
  (params (DeltaSeconds :type Float%20%28single-precision%29))
  (bind _returnvalue (Components|GetOwner))
  ;[1 1 1] This is an Actor Component, this means that it can be added to any BP Actor just like you would add a static mesh to an Actor.
  ;
  ; This class in particular is used to scroll things along the level such as the floor, pickups and obstacles
  ;;[0.375 0.8894 1] Then we add an actor local offet to "this" actor (aka whatever this component is added to), we're using delta seconds so we're not making it frame rate dependant
  (bind _output_get (Variables|Default|SetDelta%20Seconds DeltaSeconds))
  (bind _output_get_2 (Variables|Default|SetMovement (* (* (Transformation|GetActorForwardVector _returnvalue) (Variables|/Game/RunnerFiles/Blueprints/Level/BP_LevelManager.BP_LevelManager_C|GetLevelSpeed (Variables|Default|GetLevelManagerRef))) _output_get)))
  (Transformation|AddActorLocalOffset _returnvalue _output_get_2 false false))